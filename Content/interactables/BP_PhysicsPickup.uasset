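; BP_PhysicsPickup is an interactable physics object that the player can pick up and drop through interface events.
; On interact, if the player is not already holding something, it sets IsHolding, disables the Sphere's physics and collision, and snaps it to the player's ArrowHolding component.
; On drop, it detaches the actor and re-enables collision and physics, without resetting the player's IsHolding flag itself.
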(event `/Game/interfaces/Interface_Interact.INT_Interact`
  (params (PlayerRef :type "/Game/Player/BP_PlayerChar Object Reference"))
  (if (not (`/Game/Player/BP_PlayerChar.isHolding?` PlayerRef))
    (set `/Game/Player/BP_PlayerChar.isHolding?` true PlayerRef)
    (`PrimitiveComponent.SetSimulatePhysics` (`self.Sphere`) false)
    (`PrimitiveComponent.SetCollisionEnabled` (`self.Sphere`) "NoCollision")
    (`SceneComponent.K2_AttachToComponent` (`self.Sphere`) (`/Game/Player/BP_PlayerChar.arrow_holding` PlayerRef) "None" "SnapToTarget" "KeepRelative" "KeepRelative" true)))

(event `/Game/interfaces/Interface_Interact.INT_Drop`
  (bind _sphere (`self.Sphere`))
  (`self.K2_DetachFromActor` "KeepRelative" "KeepWorld" "KeepWorld")
  (`PrimitiveComponent.SetCollisionEnabled` _sphere "QueryAndPhysics")
  (`PrimitiveComponent.SetSimulatePhysics` _sphere true))

(fn `UserConstructionScript`)