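; BP_Wall is an interactable colored wall that toggles between open and closed when its OpenWall event is called.
; A FlipFlop alternately plays and reverses a Timeline, whose alpha lerps the Cube's relative Z to raise and lower it.
; The construction script gives the Cube a dynamic instance of MAT_Color and sets its color from PickupColor.
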(event `OpenWall`
  (`/Engine/EditorBlueprintResources/StandardMacros.FlipFlop`
    (:`A`
      (bind (_direction _alpha) (`Timeline|Timeline` :!label _label)
        (:`Update`
          (`SceneComponent.K2_SetRelativeLocation` (`self.Cube`) (`KismetMathLibrary.MakeVector` 0.0 0.0 (`KismetMathLibrary.Lerp` 0.0 100.0 _alpha)) false false))))
    (:`B`
      (goto _label :!via `Reverse`))))

(fn `UserConstructionScript`
  (bind _returnvalue (`PrimitiveComponent.CreateDynamicMaterialInstance` (`self.Cube`) 0 "/Game/interactables/AnimatedInteractibles/MAT_Color.MAT_Color" "None"))
  (bind _output_get (set `self.colorDMI` _returnvalue))
  (`MaterialInstanceDynamic.SetVectorParameterValue` _output_get "color" (`self.PickupColor`)))